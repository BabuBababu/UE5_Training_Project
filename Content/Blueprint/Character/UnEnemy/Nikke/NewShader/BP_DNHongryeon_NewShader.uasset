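; Character Blueprint for the Nikke DNHongryeon enemy with a new shader, exposing rim light settings for its skeletal mesh.
; The construction script creates a dynamic material instance per mesh material and writes rim light angle, spread, intensity, hardness and color to it.
; Each slot is then set back to the looped source material rather than the new instance, and a second sequence branch repeats the identical pass.
; The event graph holds only empty placeholder events.
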(fn `UserConstructionScript`
  (bind __character_skeletal_mesh (`self._character_skeletal_mesh`))
  (bind __character_skeletal_mesh_2 (`self._character_skeletal_mesh`))
  (`|ExecutionSequence`
    (:`then_1`
      (for (_array_element _array_index) (`MeshComponent.GetMaterials` __character_skeletal_mesh)
        (bind _returnvalue (`PrimitiveComponent.CreateDynamicMaterialInstance` __character_skeletal_mesh _array_index _array_element "None"))
        (`MaterialInstanceDynamic.SetScalarParameterValue` _returnvalue "RimLight_Angle" (`self.RimLight_Angle`))
        (`MaterialInstanceDynamic.SetScalarParameterValue` _returnvalue "RimLight_Spread" (`self.RimLight_Spread`))
        (`MaterialInstanceDynamic.SetScalarParameterValue` _returnvalue "RimLight_Intensity" (`self.RimLight_Intensity`))
        (`MaterialInstanceDynamic.SetScalarParameterValue` _returnvalue "RimLight_Hardness" (`self.RimLight_Hardness`))
        (`MaterialInstanceDynamic.SetVectorParameterValue` _returnvalue "RimLight_Color" (`KismetMathLibrary.Conv_ColorToLinearColor` (`self.RimLight_Color`)))
        (`PrimitiveComponent.SetMaterial` __character_skeletal_mesh_2 _array_index _array_element)))
    (:`then_2`
      (for (_array_element_2 _array_index_2) (`MeshComponent.GetMaterials` __character_skeletal_mesh)
        (bind _returnvalue_2 (`PrimitiveComponent.CreateDynamicMaterialInstance` __character_skeletal_mesh _array_index_2 _array_element_2 "None"))
        (`MaterialInstanceDynamic.SetScalarParameterValue` _returnvalue_2 "RimLight_Angle" (`self.RimLight_Angle`))
        (`MaterialInstanceDynamic.SetScalarParameterValue` _returnvalue_2 "RimLight_Spread" (`self.RimLight_Spread`))
        (`MaterialInstanceDynamic.SetScalarParameterValue` _returnvalue_2 "RimLight_Intensity" (`self.RimLight_Intensity`))
        (`MaterialInstanceDynamic.SetScalarParameterValue` _returnvalue_2 "RimLight_Hardness" (`self.RimLight_Hardness`))
        (`MaterialInstanceDynamic.SetVectorParameterValue` _returnvalue_2 "RimLight_Color" (`KismetMathLibrary.Conv_ColorToLinearColor` (`self.RimLight_Color`)))
        (`PrimitiveComponent.SetMaterial` __character_skeletal_mesh_2 _array_index_2 _array_element_2)))))